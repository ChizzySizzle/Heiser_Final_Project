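; BP_Muscle_Car_Projectile is a muscle car actor that acts as a fired projectile.
; OnFired marks it as flying and destroys it after a fixed delay.
; While it is flying, a component hit on an actor tagged Ground offsets the whole actor along the car's scaled physics velocity without sweeping, then switches off the car's physics simulation.
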(event OnComponentHit(Muscle_Car)
  (params (HitComponent :type Primitive%20Component%20Object%20Reference) (OtherActor :type Actor%20Object%20Reference) (OtherComp :type Primitive%20Component%20Object%20Reference) (NormalImpulse :type Vector :default "0, 0, 0") (Hit :type Hit%20Result%20Structure%20%28by%20ref%29))
  (bind _muscle_car (Variables|Default|GetMuscle_Car))
  (if (and (Variables|Default|Getflying) (Actor|ActorHasTag OtherActor "Ground"))
    (bind _returnvalue (Physics|GetPhysicsLinearVelocity _muscle_car "None"))
    (Transformation|AddActorWorldOffset (* _returnvalue "2000.000000,2000.000000,2000.000000"))
    (Physics|SetSimulatePhysics _muscle_car false)))

(event Custom|OnFired
  (Variables|Default|Setflying true)
  (Utilities|FlowControl|Delay 18.0)
  (Actor|DestroyActor))

(fn ConstructionScript)